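; Player Blueprint that turns to face the mouse cursor and fires projectiles.
; Shows the cursor on BeginPlay, then each Tick traces under it on the Visibility channel and turns only yaw toward the hit point at a constant interpolated speed.
; The AI_Shoot input action spawns a BP_Projectile at the Scene component's world transform when started.
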(event Input|EnhancedActionEvents|EnhancedInputActionAI_Shoot
  (params (ActionValue :type Boolean) (ElapsedSeconds :type Float%20%28double-precision%29) (TriggeredSeconds :type Float%20%28double-precision%29) (InputAction :type Input%20Action%20Object%20Reference :default "/Game/ThirdPerson/Input/Actions/AI_Shoot.AI_Shoot"))
  (:Started
    (Game|SpawnActorfromClass "/Game/Blueprints/BP_Projectile.BP_Projectile_C" (Transformation|GetWorldTransform (Variables|Default|GetScene)) "Undefined" "MultiplyWithRoot" 0 0)))

(event EventBeginPlay
  (Variables|/Script/Engine.PlayerController|SetbShowMouseCursor (Game|GetPlayerController 0) true))

(event EventTick
  (params (DeltaSeconds :type Float%20%28single-precision%29))
  (bind _returnvalue (Transformation|GetActorRotation))
  (Transformation|SetActorRotation (Math|Rotator|MakeRotator (.roll _returnvalue) (.pitch _returnvalue) (.yaw (Class|KismetMathLibrary|RInterptoConstant (Transformation|GetActorRotation) (Math|Rotator|FindLookatRotation (+ "" "") (- (.ImpactPoint (Collision|BreakHitResult (.HitResult (Game|Player|GetHitResultUnderCursorbyChannel (Game|GetPlayerController 0) "TraceTypeQuery1" true)))) (Transformation|GetActorLocation))) (Utilities|Time|GetWorldDeltaSeconds) (Variables|Default|GetInterpRotationSpeed))))))

(fn ConstructionScript)