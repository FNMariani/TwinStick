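; BP_Enemy is an AI-controlled enemy character that damages players within its attack sphere and can be killed.
; BeginPlay caches player pawns from GameState; sphere overlap starts a looping damage timer, cleared when no players remain.
; Attacks apply damage behind a resetting DoOnce cooldown and call an empty MC_EnemyAttack event.
; Incoming damage briefly halts movement and reduces health; death stops the AI, detaches the controller and destroys the actor.
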(event OnComponentBeginOverlap(AttackCollisionSphere)
  (params (OverlappedComponent :type Primitive%20Component%20Object%20Reference) (OtherActor :type Actor%20Object%20Reference) (OtherComp :type Primitive%20Component%20Object%20Reference) (OtherBodyIndex :type Integer) (bFromSweep :type Boolean) (SweepResult :type Hit%20Result%20Structure%20%28by%20ref%29))
  (Variables|Default|SetPlayerToDamage OtherActor)
  (bind _returnvalue (Utilities|Time|SetTimerbyFunctionName 0 "DamagePlayer" 1.0 true))
  (Variables|Default|SetDamagePlayerTimerReference _returnvalue)
  (CallFunction|DamagePlayer))

(event OnComponentEndOverlap(AttackCollisionSphere)
  (params (OverlappedComponent :type Primitive%20Component%20Object%20Reference) (OtherActor :type Actor%20Object%20Reference) (OtherComp :type Primitive%20Component%20Object%20Reference) (OtherBodyIndex :type Integer))
  (if (Utilities|Array|IsEmpty (Collision|GetOverlappingActors (Variables|Default|GetAttackCollisionSphere) "/Game/Player/BP_Player.BP_Player_C" :!class /Script/Engine.PrimitiveComponent))
    (Utilities|Time|ClearandInvalidateTimerbyHandle (Variables|Default|GetDamagePlayerTimerReference))))

(event Custom|MC_EnemyAttack)

(event Custom|DamagePlayer
  (Utilities|FlowControl|DoOnce false :!label _label
    (:Completed
      (if (not (Variables|Default|GetIsDead))
        (Game|Damage|ApplyDamage (Variables|Default|GetPlayerToDamage) (Variables|Default|GetDamage) 0 self)
        (CallFunction|MCEnemyAttack)
        (Utilities|FlowControl|RetriggerableDelay 0.9)
        (goto _label Reset)))))

(event EventBeginPlay
  (for _array_element (Variables|/Script/Engine.GameStateBase|GetPlayerArray (Game|GetGameState))
    (Utilities|FlowControl|Sequence
      (:then_0
        (bind _asbp_player (Utilities|Casting|CastToBP_Player (Variables|/Script/Engine.PlayerState|GetPawnPrivate _array_element)))
        (Utilities|Array|Add (Variables|Default|GetPlayerArray) _asbp_player)))))

(event Collision|EventActorBeginOverlap
  (params (OtherActor :type Actor%20Object%20Reference)))

(event EventTick
  (params (DeltaSeconds :type Float%20%28single-precision%29)))

(event Game|Damage|EventAnyDamage
  (params (Damage :type Float%20%28single-precision%29) (DamageType :type Damage%20Type%20Object%20Reference) (InstigatedBy :type Controller%20Object%20Reference) (DamageCauser :type Actor%20Object%20Reference))
  (bind _basecontrollerreference (Variables|Default|GetBaseControllerReference))
  (Class|NavMovementComponent|StopMovementKeepPathing (Variables|Character|GetCharacterMovement)) ; simulate impact of hit
  (bind _output_get (Variables|Default|SetHealth (- (Variables|Default|GetHealth) Damage)))
  (if (<= _output_get 0.0)
    (Utilities|FlowControl|DoOnce false
      (:Completed
        (Variables|Default|SetIsDead true)
        (Components|Movement|StopMovementImmediately (Variables|Character|GetCharacterMovement))
        (AI|Navigation|StopMovement _basecontrollerreference)
        (Default|EndAI _basecontrollerreference)
        (Class|Pawn|DetachfromControllerPendingDestroy)
        (Actor|DestroyActor)))))

(fn ConstructionScript)