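; Player controller for the lobby that sets up the lobby menu widget when play begins.
; For the local player it clears all existing widgets, then creates or reuses a WBP_LobbyMenu stored as PlayerHud and adds it to the viewport.
; Input starts as game-only and switches to Game and UI with the menu focused once it is shown.
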(event EventBeginPlay
  (Input|SetInputModeGameOnly self false)
  (if (Pawn|IsLocalPlayerController)
    (Viewport|RemoveAllWidgets)
    (bind _playerhud (Variables|Default|GetPlayerHud)
      (:then
        (if (not (UserInterface|Viewport|IsinViewport _playerhud))
          (UserInterface|Viewport|AddtoViewport (stale _output_get) 0 :!label _label)
          (Input|SetInputModeGameandUI self (Variables|Default|GetPlayerHud) "DoNotLock" false false)))
      (:else
        (bind _returnvalue (UserInterface|CreateWidget "/Game/Blueprints/Widgets/WBP_LobbyMenu.WBP_LobbyMenu_C" self))
        (bind _output_get (Variables|Default|SetPlayerHud _returnvalue))
        (goto _label)))))

(fn ConstructionScript)