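; Extraction point actor with a box trigger that tracks which players are inside an extraction zone and displays a preparation percentage.
; Player overlaps notify the BP_GM game mode of entries and exits and adjust its count of players in the zone.
; Entry also fires PlayerEnterInExtractionPoint.
; Tick refreshes the percentage text from a number that this graph only reads.
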(event OnComponentBeginOverlap(Box)
  (params (OverlappedComponent :type Primitive%20Component%20Object%20Reference) (OtherActor :type Actor%20Object%20Reference) (OtherComp :type Primitive%20Component%20Object%20Reference) (OtherBodyIndex :type Integer) (bFromSweep :type Boolean) (SweepResult :type Hit%20Result%20Structure%20%28by%20ref%29))
  (bind _asbp_player (Utilities|Casting|CastToBP_Player OtherActor))
  (Development|PrintString "EnterColission")
  (Default|CallPlayerEnterinExtractionPoint)
  (bind _asbp_gm (Utilities|Casting|CastToBP_GM (Game|GetGameMode)))
  (Default|PlayerEnterExtractionPoint _asbp_gm _asbp_player)
  (Math|Integer|IncrementInt (Variables|/Game/Blueprints/BP_GM.BP_GM_C|GetPlayersInExtractionPointQty _asbp_gm)))

(event OnComponentEndOverlap(Box)
  (params (OverlappedComponent :type Primitive%20Component%20Object%20Reference) (OtherActor :type Actor%20Object%20Reference) (OtherComp :type Primitive%20Component%20Object%20Reference) (OtherBodyIndex :type Integer))
  (bind _asbp_player (Utilities|Casting|CastToBP_Player OtherActor))
  (Development|PrintString "ExitColission")
  (bind _asbp_gm (Utilities|Casting|CastToBP_GM (Game|GetGameMode)))
  (Default|PlayerExitExtractionPoint _asbp_gm _asbp_player)
  (Math|Integer|DecrementInt (Variables|/Game/Blueprints/BP_GM.BP_GM_C|GetPlayersInExtractionPointQty _asbp_gm)))

(event EventBeginPlay)

(event Collision|EventActorBeginOverlap
  (params (OtherActor :type Actor%20Object%20Reference)))

(event EventTick
  (params (DeltaSeconds :type Float%20%28single-precision%29))
  (Rendering|Components|TextRender|SetText (Variables|Default|GetPreparationPercentage) (Utilities|Text|ToText(String) (Utilities|String|Append (Utilities|String|ToString(Text) (Utilities|Text|ToText(Integer) (Variables|Default|GetPreparationPercentageNumber))) "%"))))

(fn ConstructionScript)