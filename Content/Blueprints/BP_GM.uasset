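; BP_GM manages a timed match with an extraction phase, pushing updates to the HUD of every BP_Player found at BeginPlay.
; Tick updates the remaining match time, then shows go-to text once it runs out.
; Enter and exit events toggle the extraction countdown, which runs even before time expires and never resets.
; Extraction text appears only after time expires, and a finished countdown reports success on all HUDs.
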(event Custom|PlayerExitExtractionPoint
  (Variables|Default|SetbIsPlayerInExtractionPoint false)
  (for _array_element (Variables|Default|GetPlayersArray)
    (Default|HideExtractionText (Variables|/Game/Player/BP_Player.BP_Player_C|GetPlayerHUD _array_element))))

(event Custom|PlayerEnterExtractionPoint
  (Variables|Default|SetbIsPlayerInExtractionPoint true)
  (if (Variables|Default|GetbMatchTimeOver)
    (for _array_element (Variables|Default|GetPlayersArray)
      (Default|ShowExtractionText (Variables|/Game/Player/BP_Player.BP_Player_C|GetPlayerHUD _array_element)))))

(event EventTick
  (params (DeltaSeconds :type Float%20%28single-precision%29))
  (bind _returnvalue (Utilities|Time|GetTimeSeconds))
  (bind _matchtime (Variables|Default|GetMatchTime))
  (bind _returnvalue_2 (- _matchtime _returnvalue))
  (Utilities|FlowControl|Sequence
    (:then_0
      (if (not (Variables|Default|GetbMatchTimeOver))
        (for _array_element (Variables|Default|GetPlayersArray)
          (Default|UpdateMatchTime (Variables|/Game/Player/BP_Player.BP_Player_C|GetPlayerHUD _array_element) (Class|KismetTextLibrary|AsTimespanTimespan (Math|Timespan|FromSeconds _returnvalue_2))))
        (if (<= _returnvalue_2 0.0)
          (Variables|Default|SetbMatchTimeOver true)
          (for _array_element_2 (Variables|Default|GetPlayersArray)
            (Default|ShowGotoText (Variables|/Game/Player/BP_Player.BP_Player_C|GetPlayerHUD _array_element_2))))))
    (:then_1
      (if (Variables|Default|GetbIsPlayerInExtractionPoint)
        (bind _output_get (Variables|Default|SetExtractionTime (- (Variables|Default|GetExtractionTime) DeltaSeconds)))
        (if (<= _output_get 0.0)
          (Variables|Default|SetbIsPlayerInExtractionPoint false)
          (for _array_element_3 (Variables|Default|GetPlayersArray)
            (Default|ExtractionSuccessful (Variables|/Game/Player/BP_Player.BP_Player_C|GetPlayerHUD _array_element_3))
            (Development|PrintString "PlayerExtracted")))))))

(event EventBeginPlay
  (bind _outactors (Actor|GetAllActorsOfClass "/Game/Player/BP_Player.BP_Player_C"))
  (Variables|Default|SetPlayersArray _outactors))

(fn ConstructionScript)