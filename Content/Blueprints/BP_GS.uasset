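; BP_GS is a game state that relays match and extraction UI updates to every player in an extraction-style match.
; Each custom event loops over PlayerArray, casts each pawn to BP_Player and calls the matching function on it.
; The relayed messages cover the match timer, waiting for players, the go-to prompt, and extraction prompts, success and failure.
; BeginPlay, Tick and the construction script do nothing.
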(event Custom|UpdateMatchTimer
  (params (MatchTime :type Float%20%28double-precision%29))
  (for _array_element (Variables|Default|GetPlayerArray)
    (bind _asbp_player (Utilities|Casting|CastToBP_Player (PlayerState|GetPawn _array_element)))
    (Default|UpdateMatchTimer _asbp_player MatchTime)))

(event Custom|ShowGoToText
  (for _array_element (Variables|Default|GetPlayerArray)
    (bind _asbp_player (Utilities|Casting|CastToBP_Player (PlayerState|GetPawn _array_element)))
    (Default|ShowGotoText _asbp_player)))

(event Custom|ShowExtractionText
  (for _array_element (Variables|Default|GetPlayerArray)
    (bind _asbp_player (Utilities|Casting|CastToBP_Player (PlayerState|GetPawn _array_element)))
    (Default|ShowExtractionText _asbp_player)))

(event Custom|ShowExtractionSuccessful
  (for _array_element (Variables|Default|GetPlayerArray)
    (bind _asbp_player (Utilities|Casting|CastToBP_Player (PlayerState|GetPawn _array_element)))
    (Default|ShowExtractionSuccessful _asbp_player)))

(event Custom|WaitingForPlayers
  (for _array_element (Variables|Default|GetPlayerArray)
    (bind _asbp_player (Utilities|Casting|CastToBP_Player (PlayerState|GetPawn _array_element)))
    (Default|WaitingforPlayers _asbp_player)))

(event Custom|HideExtractionText
  (for _array_element (Variables|Default|GetPlayerArray)
    (bind _asbp_player (Utilities|Casting|CastToBP_Player (PlayerState|GetPawn _array_element)))
    (Default|HideExtractionText _asbp_player)))

(event Custom|ShowExtractionFailed
  (for _array_element (Variables|Default|GetPlayerArray)
    (bind _asbp_player (Utilities|Casting|CastToBP_Player (PlayerState|GetPawn _array_element)))
    (Default|ShowExtractionFailed _asbp_player)))

(event EventBeginPlay)

(event EventTick
  (params (DeltaSeconds :type Float%20%28single-precision%29)))

(fn ConstructionScript)